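; BP_Stat models a stat whose current value is derived from a base value and a set of modifiers.
; Modifiers are added uniquely to or removed from flat and multiplier lists by type, and each change triggers a recalculation.
; Recalculation adds flat values to the base, scales by the summed multipliers as a percentage of that total when nonzero, then applies optional min or max clamping.
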(fn `Add_Modifier`
  (params (Modifier :type "/Game/Blueprints/Stats/S_Stat_Modifier Structure"))
  (switch `/Game/Blueprints/Stats/ENUM_Stat_Modifier_Type` (`.Type_8_DF18FDD14ECF08C1464A839E072CF891` (break `/Game/Blueprints/Stats/S_Stat_Modifier` Modifier))
    (:`NewEnumerator0`
      (`KismetArrayLibrary.Array_AddUnique` (`self.Flat_Modifiers`) (`local.Modifier`)))
    (:`NewEnumerator1`
      (`KismetArrayLibrary.Array_AddUnique` (`self.Multiplier_Modifiers`) (`local.Modifier`))))
  (`self.Recalculate_Value`))

(fn `Recalculate_Value`
  (locals (Current_Value_Local :type "Float (double-precision)") (Multiplier_Value_Local :type "Float (double-precision)"))
  (bind (_stat_basic_info _stat_base_value _stat_clamp_min_value _stat_min_value _stat_clamp_max_value _stat_max_value) (break `/Game/Blueprints/Stats/S_Stat_Info` (`self.Stat`)))
  (bind (_stat_basic_info_2 _stat_base_value_2 _stat_clamp_min_value_2 _stat_min_value_2) (break `/Game/Blueprints/Stats/S_Stat_Info` (`self.Stat`)))
  (bind (_stat_basic_info_3 _stat_base_value_3 _stat_clamp_min_value_3 _stat_min_value_3 _stat_clamp_max_value_2 _stat_max_value_2) (break `/Game/Blueprints/Stats/S_Stat_Info` (`self.Stat`)))
  (bind (_stat_basic_info_4 _stat_base_value_4) (break `/Game/Blueprints/Stats/S_Stat_Info` (`self.Stat`)))
  (set `local.Current_Value_Local` _stat_base_value_4)
  (set `local.Multiplier_Value_Local` 0.0)
  (for _array_element (`self.Flat_Modifiers`)
    (set `local.Current_Value_Local` (+ (break `/Game/Blueprints/Stats/S_Stat_Modifier` _array_element) (`local.Current_Value_Local`))))
  (for _array_element_2 (`self.Multiplier_Modifiers`)
    (set `local.Multiplier_Value_Local` (+ (break `/Game/Blueprints/Stats/S_Stat_Modifier` _array_element_2) (`local.Multiplier_Value_Local`))))
  (if (!= (`local.Multiplier_Value_Local`) 0.0)
    (set `local.Current_Value_Local` (* (`local.Current_Value_Local`) (/ (`local.Multiplier_Value_Local`) 100.0))))
  (if (and _stat_clamp_min_value_2 (< (`local.Current_Value_Local`) _stat_min_value_2))
    (set `local.Current_Value_Local` _stat_min_value_3)
    (elif (and _stat_clamp_max_value_2 (> (`local.Current_Value_Local`) _stat_max_value_2))
      (set `local.Current_Value_Local` _stat_max_value)))
  (set `self.Current_Value` (`local.Current_Value_Local`)))

(fn `Remove_Modifier`
  (params (Modifier :type "/Game/Blueprints/Stats/S_Stat_Modifier Structure"))
  (switch `/Game/Blueprints/Stats/ENUM_Stat_Modifier_Type` (`.Type_8_DF18FDD14ECF08C1464A839E072CF891` (break `/Game/Blueprints/Stats/S_Stat_Modifier` Modifier))
    (:`NewEnumerator0`
      (`KismetArrayLibrary.Array_RemoveItem` (`self.Flat_Modifiers`) (`local.Modifier`)))
    (:`NewEnumerator1`
      (`KismetArrayLibrary.Array_RemoveItem` (`self.Multiplier_Modifiers`) (`local.Modifier`))))
  (`self.Recalculate_Value`))