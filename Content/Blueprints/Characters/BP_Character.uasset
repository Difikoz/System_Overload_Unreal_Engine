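; Character Blueprint that tracks nearby interactable actors and lets the character interact with one of them.
; InteractionRadius overlaps add and remove actors implementing BPI_Interactable in the Interactables array.
; Interact sends InteractMessage to the first array entry, passing the character itself.
; Sprint, jump and crouch start/stop events are declared but empty.
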(event `Start_Sprint`)

(event `Stop_Sprint`)

(event `Start_Jump`)

(event `Stop_Jump`)

(event `Start_Crouch`)

(event `Stop_Crouch`)

(event `Interact`
  (if (> (`KismetArrayLibrary.Array_Length` (`self.Interactables`)) 0)
    (message `/Game/Blueprints/Interfaces/BPI_Interactable.Interact` (`|GetArrayItem` (`self.Interactables`)) self)))

(event `self.InteractionRadius.OnComponentBeginOverlap`
  (params (OverlappedComponent :type "PrimitiveComponent Object Reference") (OtherActor :type "Actor Object Reference") (OtherComp :type "PrimitiveComponent Object Reference") (OtherBodyIndex :type Integer) (bFromSweep :type Boolean) (SweepResult :type "HitResult Structure (by ref)"))
  (if (`KismetSystemLibrary.DoesImplementInterface` OtherActor "/Game/Blueprints/Interfaces/BPI_Interactable.BPI_Interactable_C")
    (`KismetArrayLibrary.Array_AddUnique` (`self.Interactables`) OtherActor)))

(event `self.InteractionRadius.OnComponentEndOverlap`
  (params (OverlappedComponent :type "PrimitiveComponent Object Reference") (OtherActor :type "Actor Object Reference") (OtherComp :type "PrimitiveComponent Object Reference") (OtherBodyIndex :type Integer))
  (if (`KismetSystemLibrary.DoesImplementInterface` OtherActor "/Game/Blueprints/Interfaces/BPI_Interactable.BPI_Interactable_C")
    (`KismetArrayLibrary.Array_RemoveItem` (`self.Interactables`) OtherActor)))

(fn `UserConstructionScript`)