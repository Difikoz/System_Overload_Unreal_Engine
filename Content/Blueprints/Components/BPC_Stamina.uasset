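; BPC_Stamina is a stamina component that stores a current value and a maximum, with functions to change each.
; ReduceValue and RestoreValue subtract from or add to the current value, clamped between zero and the maximum.
; IncreaseMaxValue adds to the maximum without clamping, while DecreaseMaxValue clamps the result between zero and the previous maximum.
; Neither maximum function updates the current value, so it can remain above a lowered maximum.
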(fn `DecreaseMaxValue`
  (params (Value :type "Float (double-precision)"))
  (set `self.Max_Value` (`KismetMathLibrary.FClamp` (- (`self.Max_Value`) Value) 0.0 (`self.Max_Value`))))

(fn `IncreaseMaxValue`
  (params (Value :type "Float (double-precision)"))
  (set `self.Max_Value` (+ (`self.Max_Value`) Value)))

(fn `ReduceValue`
  (params (Value :type "Float (double-precision)"))
  (set `self.Current_Value` (`KismetMathLibrary.FClamp` (- (`self.Current_Value`) Value) 0.0 (`self.Max_Value`)))
  (return))

(fn `RestoreValue`
  (params (Value :type "Float (double-precision)"))
  (set `self.Current_Value` (`KismetMathLibrary.FClamp` (+ (`self.Current_Value`) Value) 0.0 (`self.Max_Value`)))
  (return))