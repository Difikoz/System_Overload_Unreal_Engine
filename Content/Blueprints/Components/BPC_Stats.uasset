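; BPC_Stats is a stats component meant to hold a list of stats defined by the DT_Stats data table.
; CreateStats clears the list, reads each table row and calls RecalculateStats, which has every stat recalculate its value.
; The step adding rows to the list is unwired, so CreateStats leaves it empty.
; Modifier functions are stubs: adding only loops over the stats, and removing does nothing.
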(fn `Add_Stat_Modifier`
  (params (Modifier :type "/Game/Blueprints/Stats/S_Stat_Modifier_Creator Structure"))
  (for _ (`self.Stats`)
    _))

(fn `Create_Stats`
  (`KismetArrayLibrary.Array_Clear` (`self.Stats`))
  (bind _outrownames (`DataTableFunctionLibrary.GetDataTableRowNames` "/Game/Blueprints/Stats/DT_Stats.DT_Stats"))
  (for _array_element _outrownames
    (`|GetDataTableRow` "/Game/Blueprints/Stats/DT_Stats.DT_Stats" _array_element))
  (`self.Recalculate_Stats`))

(fn `Recalculate_Stats`
  (locals (Current_Value_Local :type "Float (double-precision)") (Multiplier_Value_Local :type "Float (double-precision)"))
  (for _array_element (`self.Stats`)
    (`/Game/Blueprints/Stats/BP_Stat.Recalculate_Value` _array_element)))

(fn `Remove_Stat_Modifier`
  (params (Modifier :type "/Game/Blueprints/Stats/S_Stat_Modifier_Creator Structure")))