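; Health component that tracks current and maximum health and a death state for its owner.
; Damage and heal functions clamp the current value between zero and the maximum, do nothing once dead, and return the dead flag.
; Damage sets that flag when health reaches zero, and nothing here clears it.
; Separate functions raise or lower the maximum without adjusting current health.
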(fn `ApplyDamage`
  (params (Value :type "Float (double-precision)"))
  (returns (Dead :type Boolean))
  (if (not (`self.Is_Dead`))
    (bind _output_get (set `self.Current_Value` (`KismetMathLibrary.FClamp` (- (`self.Current_Value`) Value) 0.0 (`self.Max_Value`))))
    (if (not (> _output_get 0.0))
      (bind _output_get_2 (set `self.Is_Dead` true))))
  (return _output_get_2))

(fn `ApplyHeal`
  (params (Value :type "Float (double-precision)"))
  (returns (Dead :type Boolean))
  (if (not (`self.Is_Dead`))
    (set `self.Current_Value` (`KismetMathLibrary.FClamp` (+ (`self.Current_Value`) Value) 0.0 (`self.Max_Value`))))
  (return (`self.Is_Dead`)))

(fn `DecreaseMaxValue`
  (params (Value :type "Float (double-precision)"))
  (set `self.Max_Value` (`KismetMathLibrary.FClamp` (- (`self.Max_Value`) Value) 0.0 (`self.Max_Value`))))

(fn `IncreaseMaxValue`
  (params (Value :type "Float (double-precision)"))
  (set `self.Max_Value` (+ (`self.Max_Value`) Value)))