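; Inventory component that stores items as an array of stacks, each holding an ID, amount and item data.
; AddItem increases the amount of a stack with a matching ID, otherwise adds a new stack using the row from DT_Items.
; The ItemFound flag is set on a match and cleared only after a new stack is added.
; RemoveItem is an empty stub with disconnected search nodes.
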(fn `Add_Item`
  (params (Item :type "Name (by ref)") (Amount :type Integer))
  (locals (ItemFound :type Boolean))
  (bind _item (`local.Item`))
  (for (_array_element _array_index) (`self.Stacks`)
    (if (== (break `/Game/Blueprints/Items/S_Item_Stack` _array_element) Item)
      (`KismetArrayLibrary.Array_Set` (`self.Stacks`) _array_index (make `/Game/Blueprints/Items/S_Item_Stack` Item (+ (`.Amount_3_C82BCDE2403737CEBE5C48B9D36113C8` (break `/Game/Blueprints/Items/S_Item_Stack` _array_element)) (`local.Amount`)) (`.Item_10_97D56CF54FF74064E20621B66D35FFA9` (break `/Game/Blueprints/Items/S_Item_Stack` _array_element))))
      (set `local.ItemFound` true)
      (break)))
  (if (not (`local.ItemFound`))
    (bind _returnvalue (`|GetDataTableRow` "/Game/Blueprints/Items/DT_Items.DT_Items" _item)
      (:`then`
        (`KismetArrayLibrary.Array_Add` (`self.Stacks`) (make `/Game/Blueprints/Items/S_Item_Stack` _item (`local.Amount`) _returnvalue))
        (set `local.ItemFound` false)))))

(fn `Remove_Item`
  (params (Item :type "Name (by ref)") (Amount :type Integer)))