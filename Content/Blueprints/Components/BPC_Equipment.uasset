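; Equipment component that manages a pawn's weapon and armor slots as maps from item type to item ID.
; Initialize stores the owning pawn and resets the slots to "None".
; Equipping looks up the item's data table row, unequips that type's slot, applies the row's stat modifiers to PawnStats and removes the item from PawnInventory.
; Unequipping removes those modifiers, returns the item to inventory and deletes the slot entry.
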(fn `Create_Armor_Slots`
  (`BlueprintMapLibrary.Map_Clear` (`self.Armor_Slots`))
  (`BlueprintMapLibrary.Map_Add` (`self.Armor_Slots`) "NewEnumerator0")
  (`BlueprintMapLibrary.Map_Add` (`self.Armor_Slots`) "NewEnumerator1")
  (`BlueprintMapLibrary.Map_Add` (`self.Armor_Slots`) "NewEnumerator2")
  (`BlueprintMapLibrary.Map_Add` (`self.Armor_Slots`) "NewEnumerator3"))

(fn `Create_Weapon_Slots`
  (`BlueprintMapLibrary.Map_Clear` (`self.Weapon_Slots`))
  (`BlueprintMapLibrary.Map_Add` (`self.Weapon_Slots`) "NewEnumerator0")
  (`BlueprintMapLibrary.Map_Add` (`self.Weapon_Slots`) "NewEnumerator0"))

(fn `Equip_Armor`
  (params (New_Armor_ID :type Name))
  (locals (Armor_Type_Local :type "/Game/Blueprints/Items/Armor/ENUM_Armor_Type Enum"))
  (bind _pawn (`self.Pawn`))
  (bind _returnvalue (`|GetDataTableRow` "/Game/Blueprints/Items/Armor/DT_Armors.DT_Armors" New_Armor_ID)
    (:`then`
      (bind (_item_info _armor_type _modifiers) (break `/Game/Blueprints/Items/Armor/S_Armor` _returnvalue))
      (bind _output_get (set `local.Armor_Type_Local` _armor_type))
      (`self.Unequip_Armor` _output_get)
      (`BlueprintMapLibrary.Map_Add` (`self.Armor_Slots`) (`local.Armor_Type_Local`) (`local.New_Armor_ID`))
      (for _array_element _modifiers
        (`/Game/Blueprints/Components/BPC_Stats.Add_Stat_Modifier` (`/Game/Blueprints/Characters/BP_Character.Pawn_Stats` _pawn) _array_element))
      (`/Game/Blueprints/Components/BPC_Inventory.Remove_Item` (`/Game/Blueprints/Characters/BP_Character.Pawn_Inventory` _pawn) (`local.New_Armor_ID`) 1 "/Game/Blueprints/Items/Armor/DT_Armors.DT_Armors")
      (return))))

(fn `Equip_Weapon`
  (params (New_Weapon_ID :type Name))
  (locals (Weapon_Type_Local :type "/Game/Blueprints/Items/Weapons/ENUM_Weapon_Type Enum"))
  (bind _pawn (`self.Pawn`))
  (bind _returnvalue (`|GetDataTableRow` "/Game/Blueprints/Items/Weapons/DT_Weapons.DT_Weapons" New_Weapon_ID)
    (:`then`
      (bind (_item_info _weapon_type _modifiers) (break `/Game/Blueprints/Items/Weapons/S_Weapon` _returnvalue))
      (bind _output_get (set `local.Weapon_Type_Local` _weapon_type))
      (`self.Unequip_Weapon` _output_get)
      (`BlueprintMapLibrary.Map_Add` (`self.Weapon_Slots`) (`local.Weapon_Type_Local`) (`local.New_Weapon_ID`))
      (for _array_element _modifiers
        (`/Game/Blueprints/Components/BPC_Stats.Add_Stat_Modifier` (`/Game/Blueprints/Characters/BP_Character.Pawn_Stats` _pawn) _array_element))
      (`/Game/Blueprints/Components/BPC_Inventory.Remove_Item` (`/Game/Blueprints/Characters/BP_Character.Pawn_Inventory` _pawn) (`local.New_Weapon_ID`) 1 "/Game/Blueprints/Items/Weapons/DT_Weapons.DT_Weapons")
      (return))))

(fn `Initialize`
  (params (Pawn :type "/Game/Blueprints/Characters/BP_Character Object Reference"))
  (set `self.Pawn` Pawn)
  (`self.Create_Weapon_Slots`)
  (`self.Create_Armor_Slots`))

(fn `Unequip_Armor`
  (params (Armor_Type :type "/Game/Blueprints/Items/Armor/ENUM_Armor_Type Enum" :default "NewEnumerator0"))
  (locals (Old_Armor_Local :type Name))
  (bind _pawn (`self.Pawn`))
  (bind _output_get (set `local.Old_Armor_Local` (`BlueprintMapLibrary.Map_Find` (`self.Armor_Slots`) Armor_Type)))
  (bind _returnvalue (`|GetDataTableRow` "/Game/Blueprints/Items/Armor/DT_Armors.DT_Armors" _output_get)
    (:`then`
      (for _array_element (`.Modifiers_7_907BF0E047509AB4366F71B46E1FF1F2` (break `/Game/Blueprints/Items/Armor/S_Armor` _returnvalue))
        (`/Game/Blueprints/Components/BPC_Stats.Remove_Stat_Modifier` (`/Game/Blueprints/Characters/BP_Character.Pawn_Stats` _pawn) _array_element))
      (`/Game/Blueprints/Components/BPC_Inventory.Add_Item` (`/Game/Blueprints/Characters/BP_Character.Pawn_Inventory` _pawn) (`local.Old_Armor_Local`) "NewEnumerator0" 1 "/Game/Blueprints/Items/Armor/DT_Armors.DT_Armors")
      (`BlueprintMapLibrary.Map_Remove` (`self.Armor_Slots`) (`local.Armor_Type`))
      (return))))

(fn `Unequip_Weapon`
  (params (Weapon_Type :type "/Game/Blueprints/Items/Weapons/ENUM_Weapon_Type Enum" :default "NewEnumerator0"))
  (locals (Old_Weapon_Local :type Name))
  (bind _pawn (`self.Pawn`))
  (bind _output_get (set `local.Old_Weapon_Local` (`BlueprintMapLibrary.Map_Find` (`self.Weapon_Slots`) Weapon_Type)))
  (bind _returnvalue (`|GetDataTableRow` "/Game/Blueprints/Items/Weapons/DT_Weapons.DT_Weapons" _output_get)
    (:`then`
      (for _array_element (`.Modifiers_24_ED79947C4D16681359B9C69CFF9B6621` (break `/Game/Blueprints/Items/Weapons/S_Weapon` _returnvalue))
        (`/Game/Blueprints/Components/BPC_Stats.Remove_Stat_Modifier` (`/Game/Blueprints/Characters/BP_Character.Pawn_Stats` _pawn) _array_element))
      (`/Game/Blueprints/Components/BPC_Inventory.Add_Item` (`/Game/Blueprints/Characters/BP_Character.Pawn_Inventory` _pawn) (`local.Old_Weapon_Local`) "NewEnumerator0" 1 "/Game/Blueprints/Items/Weapons/DT_Weapons.DT_Weapons")
      (`BlueprintMapLibrary.Map_Remove` (`self.Weapon_Slots`) (`local.Weapon_Type`))
      (return))))