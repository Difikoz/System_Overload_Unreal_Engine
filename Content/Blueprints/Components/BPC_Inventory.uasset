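; Inventory component that stores items as stacks keyed by item ID and data table, with functions to add and remove amounts.
; AddItem gives each Weapon or Armor unit its own stack.
; Ammo, Consumable and Resource share a top-up path for matching or new stacks, though its capacity check compares against zero.
; RemoveItem drains matching stacks from the end, deleting emptied ones and printing any shortfall.
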(fn `Add_Item`
  (params (Item_ID :type "Name (by ref)") (Item_Type :type "/Game/Blueprints/Items/ENUM_Item_Type Enum" :default "NewEnumerator0") (Amount :type Integer) (Data_Table :type "DataTable Object Reference"))
  (locals (Amount_To_Add_Local :type Integer) (Amount_In_Stack_Local :type Integer) (Stack_Index_Local :type Integer))
  (set `local.Amount_To_Add_Local` Amount)
  (switch `/Game/Blueprints/Items/ENUM_Item_Type` (`local.Item_Type`)
    (:`NewEnumerator0`
      _)
    (:`NewEnumerator4`
      _)
    (:`NewEnumerator5`
      (for (_array_element _array_index) (`self.Stacks`) :!label _label
        (set `local.Amount_In_Stack_Local` (`.Amount_3_C82BCDE2403737CEBE5C48B9D36113C8` (break `/Game/Blueprints/Items/S_Item_Stack` _array_element)))
        (set `local.Stack_Index_Local` _array_index)
        (if (and (== (break `/Game/Blueprints/Items/S_Item_Stack` _array_element) (`local.Item_ID`)) (== (`.Data_Table_14_D189DD3E4E90A0A69BC00CA471987555` (break `/Game/Blueprints/Items/S_Item_Stack` _array_element)) (`local.Data_Table`)))
          (if (< (`local.Amount_In_Stack_Local`) 0) :!label _label_2
            (`/Engine/EditorBlueprintResources/StandardMacros.IncrementInt` (`local.Amount_In_Stack_Local`)
              (:`  `
                (`/Engine/EditorBlueprintResources/StandardMacros.DecrementInt` (`local.Amount_To_Add_Local`)
                  (:`  `
                    (`KismetArrayLibrary.Array_Set` (`self.Stacks`) (`local.Stack_Index_Local`) (make `/Game/Blueprints/Items/S_Item_Stack` (`local.Item_ID`) (`local.Amount_In_Stack_Local`) (`local.Data_Table`)))
                    (if (> (`local.Amount_To_Add_Local`) 0)
                      (goto _label_2)
                      (else
                        (return))))))))))
      (while (> (`local.Amount_To_Add_Local`) 0)
        (bind _returnvalue (`KismetArrayLibrary.Array_Add` (`self.Stacks`) (make `/Game/Blueprints/Items/S_Item_Stack` (`local.Item_ID`) 0 (`local.Data_Table`))))
        (set `local.Stack_Index_Local` _returnvalue)
        (set `local.Amount_In_Stack_Local` 0)
        (goto _label_2))
      (return))
    (:`NewEnumerator2`
      (goto _label))
    (:`NewEnumerator3`
      (goto _label)))
  (while (> (`local.Amount_To_Add_Local`) 0)
    (`/Engine/EditorBlueprintResources/StandardMacros.DecrementInt` (`local.Amount_To_Add_Local`)
      (:`  `
        (`KismetArrayLibrary.Array_Add` (`self.Stacks`) (make `/Game/Blueprints/Items/S_Item_Stack` (`local.Item_ID`) 1 (`local.Data_Table`))))))
  (return))

(fn `Remove_Item`
  (params (Item_ID :type "Name (by ref)") (Amount :type Integer) (Data_Table :type "DataTable Object Reference"))
  (locals (Amount_To_Remove_Local :type Integer) (Amount_In_Stack_Local :type Integer) (Stack_Index_Local :type Integer))
  (set `local.Amount_To_Remove_Local` Amount)
  (bind (_arrayindex _arrayelement) (`/Engine/EditorBlueprintResources/StandardMacros.ReverseForEachLoop` (`self.Stacks`))
    (:`LoopBody`
      (set `local.Stack_Index_Local` _arrayindex)
      (set `local.Amount_In_Stack_Local` (`.Amount_3_C82BCDE2403737CEBE5C48B9D36113C8` (break `/Game/Blueprints/Items/S_Item_Stack` _arrayelement)))
      (if (and (== (break `/Game/Blueprints/Items/S_Item_Stack` _arrayelement) (`local.Item_ID`)) (== (`.Data_Table_14_D189DD3E4E90A0A69BC00CA471987555` (break `/Game/Blueprints/Items/S_Item_Stack` _arrayelement)) (`local.Data_Table`)))
        (if (> (`local.Amount_In_Stack_Local`) 0)
          (`/Engine/EditorBlueprintResources/StandardMacros.DecrementInt` (`local.Amount_In_Stack_Local`) :!label _label
            (:`  `
              (`/Engine/EditorBlueprintResources/StandardMacros.DecrementInt` (`local.Amount_To_Remove_Local`)
                (:`  `
                  (if (> (`local.Amount_In_Stack_Local`) 0)
                    (`KismetArrayLibrary.Array_Set` (`self.Stacks`) (`local.Stack_Index_Local`) (make `/Game/Blueprints/Items/S_Item_Stack` (`local.Item_ID`) (`local.Amount_In_Stack_Local`) (`local.Data_Table`)))
                    (if (> (`local.Amount_To_Remove_Local`) 0)
                      (goto _label)
                      (else
                        (return)))
                    (else
                      (`KismetArrayLibrary.Array_Remove` (`self.Stacks`) (`local.Stack_Index_Local`)))))))))))
    (:`Completed`
      (if (> (`local.Amount_To_Remove_Local`) 0)
        (`KismetSystemLibrary.PrintText` (`|FormatText` "Cant Remove {amount} {item}" (`local.Amount_To_Remove_Local`) (`local.Item_ID`)))
        (return)
        (else
          (return))))))